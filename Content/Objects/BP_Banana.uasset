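; BP_Banana is a clickable banana actor that signals the robot to go for it.
; Clicking its static mesh stores the clicked component's owner in ChosenBananaRef and sets the "bGoingForBanana?" Blackboard key through BP_RobotCtrl.
; GoingForBanana is an empty event.
; An unconnected AIMoveTo chain that would move BP_Robot to the banana and attach the banana when close never runs.
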(event `self.StaticMesh.OnClicked`
  (params (TouchedComponent :type "PrimitiveComponent Object Reference") (ButtonPressed :type "Key Structure"))
  (set `self.ChosenBananaRef` (`ActorComponent.GetOwner` TouchedComponent))
  (bind _returnvalue (`GameplayStatics.GetActorOfClass` "/Game/AI/AI_Logic/BP_RobotCtrl.BP_RobotCtrl_C"))
  (`BlackboardComponent.SetValueAsBool` (`AIBlueprintHelperLibrary.GetBlackboard` _returnvalue) "bGoingForBanana?" true))

(event `GoingForBanana`
  ;[0.03854 0.03854 0.03854] Робот направляется за бананом
)

(fn `UserConstructionScript`)