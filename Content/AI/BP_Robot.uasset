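; BP_Robot is an AI companion that continually follows the player character.
; From BeginPlay, FollowPlayer runs AI Move To toward the player and calls itself again after a short delay on success.
; On failure it waits, then teleports beside the player at a fixed world-X offset and resumes following if not already close.
; If the robot is close after a failure, the follow loop ends.
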(event `self.ReceiveBeginPlay`
  (`self.FollowPlayer`))

(event `FollowPlayer`
  (`|AIMoveTo` self (0.0 0.0 0.0) (`GameplayStatics.GetPlayerCharacter` 0) 10.0
    (:`OnSuccess`
      (`KismetSystemLibrary.Delay` 0.1)
      (`self.FollowPlayer`))
    (:`OnFail`
      (`KismetSystemLibrary.Delay` 3.0)
      (if (> (`self.GetDistanceTo` (`GameplayStatics.GetPlayerCharacter` 0)) 50.0)
        (`self.K2_SetActorLocation` self (+ (`self.K2_GetActorLocation` (`GameplayStatics.GetPlayerCharacter` 0)) (150.0 0.0 0.0)) false true)
        (`KismetSystemLibrary.Delay` 0.2)
        (`self.FollowPlayer`)))))

(fn `UserConstructionScript`)